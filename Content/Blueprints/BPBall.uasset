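; BPBall is the physical ball for Pocket League, a car-ball game; on BeginPlay it registers with GM_PocketLeague and collects all Chaos vehicles as trace-ignored actors.
; Each tick a downward line trace places two ground decals under the ball, scaling one by height, and stretches a vertical guide line between ball and ground when high up.
; It also converts ball velocity to km/h to switch four Niagara effects on above a speed threshold.
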(event `self.ReceiveBeginPlay`
  (`|ExecutionSequence`
    (:`then_0`
      ;[1 1 1] Adding Self To Game Mode
      (bind _asgm_pocket_league (cast `/Game/Blueprints/GM_PocketLeague` (`GameplayStatics.GetGameMode`)))
      (bind _output_get (set `self.As GM Pocket League` _asgm_pocket_league))
      (`KismetArrayLibrary.Array_Add` (`/Game/Blueprints/GM_PocketLeague.Balls` _output_get) self))
    (:`then_1`
      ;[1 1 1] Ignored Actors
      (bind _outactors (`GameplayStatics.GetAllActorsOfClass` "/Game/VehicleAdvBP/Blueprints/ChaosVehicleBlueprint.ChaosVehicleBlueprint_C"))
      (for _array_element _outactors
        (`KismetArrayLibrary.Array_Add` (`self.IgnoredActors`) _array_element)))))

(event `self.ReceiveTick`
  (params (DeltaSeconds :type "Float (single-precision)"))
  (bind _niagara1 (`self.Niagara1`))
  (bind _returnvalue (`SceneComponent.K2_GetComponentLocation` (`self.Ball`)))
  (`|ExecutionSequence`
    (:`then_0`
      ;[1 1 1] Ball Decals and Line
      (bind (_outhit _returnvalue_2) (`KismetSystemLibrary.LineTraceSingle` _returnvalue (`KismetMathLibrary.MakeVector` (.x _returnvalue) (.y _returnvalue) -500.0) "TraceTypeQuery1" false (`self.IgnoredActors`)))
      (if _returnvalue_2
        (bind (_bblockinghit _binitialoverlap _time _distance _location) (`GameplayStatics.BreakHitResult` _outhit))
        (bind _output_get (set `self.GroundLocation` _location))
        (`SceneComponent.K2_SetWorldLocation` (`self.Decal2`) _output_get false false)
        (`SceneComponent.K2_SetWorldLocation` (`self.Decal1`) _output_get false false)
        (bind _returnvalue_3 (`KismetMathLibrary.FClamp` (/ 100.0 _distance) 0.0 0.4))
        (`SceneComponent.SetWorldScale3D` (`self.Decal2`) (`KismetMathLibrary.MakeVector` 0.1 _returnvalue_3 _returnvalue_3))
        (if (> _distance 300.0)
          (`SceneComponent.SetVisibility` (`self.Line`) true false)
          (`SceneComponent.K2_SetWorldLocation` (`self.Line`) (/ (+ (`SceneComponent.K2_GetComponentLocation` (`self.Ball`)) (`self.GroundLocation`)) (2.0 2.0 2.0)) false false)
          (`SceneComponent.SetWorldScale3D` (`self.Line`) (`KismetMathLibrary.MakeVector` 0.01 0.01 (/ _distance 100.0)))
          (else
            (`SceneComponent.SetVisibility` (`self.Line`) false false)))))
    (:`then_1`
      ;[1 1 1] Render Particles Based On Ball Speed
      (set `self.BallSpeed` (`KismetMathLibrary.FFloor` (`KismetMathLibrary.Abs` (* (`KismetMathLibrary.VSize` (`SceneComponent.GetComponentVelocity` (`self.Ball`))) 0.036))))
      (if (> (`self.BallSpeed`) 40)
        (`ActorComponent.Activate` _niagara1 false)
        (`ActorComponent.Activate` (`self.Niagara2`) false)
        (`ActorComponent.Activate` (`self.Niagara3`) false)
        (`ActorComponent.Activate` (`self.Niagara`) false)
        (else
          (`ActorComponent.Deactivate` _niagara1)
          (`ActorComponent.Deactivate` (`self.Niagara2`))
          (`ActorComponent.Deactivate` (`self.Niagara3`))
          (`ActorComponent.Deactivate` (`self.Niagara`)))))))

(fn `UserConstructionScript`)