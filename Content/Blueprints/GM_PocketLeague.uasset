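; GM_PocketLeague is the Pocket League game mode Blueprint that runs the match countdown clock.
; On BeginPlay it adds the HUD widget to the first player's viewport and starts UpdateTime after a short delay.
; While IsPlaying, a looping one-second Delay decrements the minutes and seconds and refreshes the HUD.
; When time runs out, it prints "GAME OVER" and clears IsPlaying, ending the loop.
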(event `self.ReceiveBeginPlay`
  (bind _returnvalue (`|CreateWidget` "/Game/Blueprints/HUD_UI.HUD_UI_C" (`GameplayStatics.GetPlayerController` 0)))
  (bind _output_get (set `self.HUD_UI` _returnvalue))
  (`UserWidget.AddToViewport` _output_get 0)
  (`KismetSystemLibrary.Delay` 1.0)
  (`self.Update Time`))

(event `Update Time`
  ;[1 1 1] Update Time
  (if (`self.IsPlaying`) :!label _label
    (if (<= (`self.TimeSeconds`) 0)
      (if (<= (`self.TimeMinutes`) 0)
        (`KismetSystemLibrary.PrintString` "GAME OVER" true true (struct :`R` 0.952433 :`G` 1.0 :`B` 0.884944 :`A` 1.0) 5.0)
        (set `self.IsPlaying` false)
        (else
          (`/Engine/EditorBlueprintResources/StandardMacros.DecrementInt` (`self.TimeMinutes`)
            (:`  `
              (set `self.TimeSeconds` 59)
              (`/Game/Blueprints/HUD_UI.Update HUD Time` (`self.HUD_UI`) :!label _label_2)
              (`KismetSystemLibrary.Delay` 1.0)
              (goto _label)))))
      (else
        (`/Engine/EditorBlueprintResources/StandardMacros.DecrementInt` (`self.TimeSeconds`)
          (:`  `
            (goto _label_2)))))))

(event `self.ReceiveTick`
  (params (DeltaSeconds :type "Float (single-precision)")))

(fn `UserConstructionScript`)